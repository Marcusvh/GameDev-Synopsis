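; Readable paper pickup that shows a lore widget when the player interacts inside its linked trigger box.
; Overlap shows an interact prompt and opens a gate, letting Tick poll a short-lived flag set on Interact release.
; The first read plays a paper sound and opens a second gate, so a later release destroys paper and trigger, clears widgets and prints the page count.
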(event Custom|OnActorBeginOverlap_Event
  (params (OverlappedActor :type Actor%20Object%20Reference) (OtherActor :type Actor%20Object%20Reference))
  (bind _lifespantest (Variables|Default|GetLifespanTest))
  (bind _triggerbox (Variables|Default|GetTriggerBox))
  (Utilities|Casting|CastToBP_FirstPersonCharacter OtherActor)
  (bind _returnvalue (UserInterface|CreateWidget "/Game/FirstPerson/Blueprints/PressToInteract.PressToInteract_C"))
  (UserInterface|Viewport|AddtoViewport _returnvalue 0)
  (Utilities|FlowControl|Gate true) ; enters at Open
)

(event Custom|OnActorEndOverlap_Event
  (params (OverlappedActor :type Actor%20Object%20Reference) (OtherActor :type Actor%20Object%20Reference))
  (bind _lifespantest (Variables|Default|GetLifespanTest))
  (bind _triggerbox (Variables|Default|GetTriggerBox))
  (Viewport|RemoveAllWidgets)
  (Utilities|FlowControl|Gate true) ; enters at Close
)

(event Collision|EventActorBeginOverlap
  (params (OtherActor :type Actor%20Object%20Reference)))

(event EventTick
  (params (DeltaSeconds :type Float%20%28single-precision%29))
  (bind _lifespantest (Variables|Default|GetLifespanTest))
  (bind _triggerbox (Variables|Default|GetTriggerBox))
  (Utilities|FlowControl|Gate true
    (:Exit
      (if (stale Input|ActionEvents|InputActionInterract _output_get)
        (bind _returnvalue (UserInterface|CreateWidget "/Game/FirstPerson/Blueprints/PaperLore.PaperLore_C"))
        (Viewport|RemoveAllWidgets)
        (UserInterface|Viewport|AddtoViewport _returnvalue 0)
        ;[1 1 1] SCUFFED
        (Utilities|FlowControl|DoOnce false
          (:Completed
            (Audio|PlaySound2D (Variables|Default|GetPaperSound) 1.0 1.0 0.0 0 0)
            (Utilities|FlowControl|Gate true) ; enters at Open
          ))))))

(event EventBeginPlay
  (bind _triggerbox (Variables|Default|GetTriggerBox))
  (EventDispatchers|AssignOnActorBeginOverlap _triggerbox (delegate Custom|OnActorBeginOverlap_Event))
  (EventDispatchers|AssignOnActorEndOverlap _triggerbox (delegate Custom|OnActorEndOverlap_Event))
  (Input|EnableInput (Game|GetPlayerController 0))
  (Variables|Default|SetPaperSound "/Game/Movies/Sounds/sfx-paperflip4.sfx-paperflip4"))

(event Input|ActionEvents|InputActionInterract
  (params (Key :type Key%20Structure :default "None"))
  (bind _triggerbox (Variables|Default|GetTriggerBox))
  (:Pressed
    (Variables|Default|SetLifespanTest 0.1))
  (:Released
    ;[1 1 1] SCUFFED
    (Utilities|FlowControl|Gate true
      (:Exit
        (Actor|SetLifeSpan (Variables|Default|GetLifespanTest))
        (Actor|SetLifeSpan _triggerbox (Variables|Default|GetLifespanTest))
        (Actor|DestroyActor)
        (Actor|DestroyActor _triggerbox)
        (Viewport|RemoveAllWidgets)
        (bind _returnvalue (Class|MyBlueprintFunctionLibrary|AmountOfPages))
        (Development|PrintString _returnvalue)))))

(event Input|ActionEvents|InputActionInterract
  (params (Key :type Key%20Structure :default "None"))
  (:Released
    (bind _output_get (Variables|Default|SetHasInterracted true))
    (Utilities|FlowControl|Delay 0.2)
    (Variables|Default|SetHasInterracted false)))

(fn ConstructionScript)